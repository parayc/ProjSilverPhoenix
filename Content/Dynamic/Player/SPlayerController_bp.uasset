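; Player controller Blueprint that manages the player's HUD, death screen and inventory screen.
; BeginPlay adds the player UI, and OnDeath shows the death UI with the mouse cursor.
; The Inventory input toggles a lazily created, reused widget, switching cursor visibility and input between game-only and game-and-UI.
; The Inventory's OnUpdateRequest event refreshes individual widget slots by index.
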(event OnUpdateRequest(Inventory)
  (params (Index :type Integer))
  (bind _inventorywidget (Variables|Default|GetInventoryWIDGET))
  (Utilities|IsValid _inventorywidget
    (:Is%20Valid
      (Default|UpdateSlotatIndex _inventorywidget Index))))

(event Custom|OnDeath
  (bind _returnvalue (UserInterface|CreateWidget "/Game/Dynamic/UI/Death_UI.Death_UI_C"))
  (UserInterface|Viewport|AddtoViewport _returnvalue 0)
  (Variables|Default|SetbShowMouseCursor true))

(event EventBeginPlay
  (bind _returnvalue (UserInterface|CreateWidget "/Game/Dynamic/UI/Player_UI.Player_UI_C"))
  (bind _output_get (Variables|Default|SetPlayer_UIWidget _returnvalue))
  (UserInterface|Viewport|AddtoViewport _output_get 0))

(event EventTick
  (params (DeltaSeconds :type Float%20%28single-precision%29)))

(event Input|ActionEvents|InputActionInventory
  (params (Key :type Key%20Structure))
  (:Pressed
    (if (Variables|Default|GetIsInventoryVisible)
      (CallFunction|RemoveInventoryWidget)
      (else
        (CallFunction|AddInventoryWidget self)))))

(fn ConstructionScript)

(fn AddInventoryWidget
  (params (Target :type Player%20Controller%20Object%20Reference))
  (Utilities|IsValid (Variables|Default|GetInventoryWIDGET)
    (:Is%20Valid
      _)
    (:Is%20Not%20Valid
      (bind _returnvalue (UserInterface|CreateWidget "/Game/Dynamic/UI/Inventory.Inventory_C" self (Variables|Default|GetInventory)))
      (bind _output_get (Variables|Default|SetInventoryWIDGET _returnvalue))))
  (UserInterface|Viewport|AddtoViewport _output_get 0)
  (Input|SetInputModeGameandUI Target (Variables|Default|GetInventoryWIDGET) "DoNotLock" true)
  (Variables|Default|SetbShowMouseCursor true)
  (Variables|Default|SetIsInventoryVisible true))

(fn RemoveInventoryWidget
  (Input|SetInputModeGameOnly self)
  (Widget|RemovefromParent (Variables|Default|GetInventoryWIDGET))
  (Variables|Default|SetbShowMouseCursor false)
  (Variables|Default|SetIsInventoryVisible false))