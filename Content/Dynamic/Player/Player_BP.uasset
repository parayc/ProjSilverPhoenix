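; Player character Blueprint that handles startup setup and the response to death.
; On BeginPlay it binds the death request, sets game-only input with a hidden cursor, and enables physics on mesh bodies below a clothing bone for secondary motion.
; A death request triggers the DarkKnightAnim death event, then notifies SPlayerController_bp.
; Tick is empty, and experimental enemy distance, view-angle and line-of-sight checks are left disconnected.
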(event Custom|OnDeathRequest_Event_0
  (bind _asdark_knight_anim (Utilities|Casting|CastToDarkKnightAnim (Components|SkeletalMesh|GetAnimInstance (Variables|Character|GetMesh))))
  (Default|DeathEvent _asdark_knight_anim)
  (bind _assplayer_controller_bp (Utilities|Casting|CastToSPlayerController_bp (Pawn|GetController)))
  (Default|OnDeath _assplayer_controller_bp))

(event EventBeginPlay
  (EventDispatchers|AssignOnDeathRequest (delegate Custom|OnDeathRequest_Event_0))
  (bind _asplayer_controller (Utilities|Casting|CastToPlayerController (Pawn|GetController)))
  (Input|SetInputModeGameOnly _asplayer_controller)
  (Variables|/Script/Engine.PlayerController|SetbShowMouseCursor _asplayer_controller false)
  (Class|SkeletalMeshComponent|SetAllBodiesBelowSimulatePhysics (Variables|Character|GetMesh) (Utilities|Name|MakeLiteralName "Clothes_f_01") true true))

(event EventTick
  (params (DeltaSeconds :type Float%20%28single-precision%29)))

(fn ConstructionScript)