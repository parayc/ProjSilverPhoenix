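; A moving platform that carries its static mesh back and forth along a spline.
; Each tick advances a clamped time value by the signed direction, then places the mesh at that spline point at constant velocity, keeping its rotation.
; Reaching either end flips the direction.
; The construction script fixes a one-second spline duration, which Tick also prints every frame.
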(event EventBeginPlay)

(event Collision|EventActorBeginOverlap
  (params (OtherActor :type Actor%20Object%20Reference)))

(event EventTick
  (params (DeltaSeconds :type Float%20%28single-precision%29))
  (bind _staticmesh (Variables|Default|GetStaticMesh))
  (bind _spline (Variables|Default|GetSpline))
  (bind _duration (Variables|/Script/Engine.SplineComponent|GetDuration _spline))
  (Variables|Default|SetDetlaTime DeltaSeconds)
  (Development|PrintString (Utilities|String|ToString(Float) _duration))
  (bind _output_get (Variables|Default|SetPlatformTime (+ (Variables|Default|GetPlatformTime) (* (Math|Conversions|ToFloat(Integer) (Variables|Default|GetDirection)) (Variables|Default|GetDetlaTime)))))
  (Variables|Default|SetPlatformTime (Math|Float|Clamp(Float) _output_get 0.0 _duration))
  (Transformation|SetWorldLocationAndRotation _staticmesh (Spline|GetLocationatTime (Variables|Default|GetSpline) (Variables|Default|GetPlatformTime) "World" true) (Transformation|GetWorldRotation _staticmesh) false false)
  (if (or (Math|Float|NearlyEqual(Float) (Variables|/Script/Engine.SplineComponent|GetDuration (Variables|Default|GetSpline)) (Variables|Default|GetPlatformTime) 1e-06) (Math|Float|NearlyEqual(Float) (Variables|Default|GetPlatformTime) 0.0 1e-06))
    (Math|Integer|CompareInt (Variables|Default|GetDirection)
      (:>
        (Variables|Default|SetDirection -1))
      (:<
        (Variables|Default|SetDirection 1)))))

(fn ConstructionScript
  (Variables|Default|SetDirection 1)
  (Variables|/Script/Engine.SplineComponent|SetDuration (Variables|Default|GetSpline) 1.0))