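; Player character Blueprint that sets up game input and handles the player's death.
; BeginPlay binds the death request delegate, switches to game-only input and hides the mouse cursor.
; On death it triggers the death animation on MeleeAnim_BP, then notifies SPlayerController_bp.
; Disconnected leftover nodes hold an enemy sight test using distance, view angle and line of sight, plus trace and rotation fragments; Tick does nothing.
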(event Custom|OnDeathRequest_Event_0
  (bind _asmelee_anim_bp (Utilities|Casting|CastToMeleeAnim_BP (Components|SkeletalMesh|GetAnimInstance (Variables|Character|GetMesh))))
  (Default|OnDeathAnimation _asmelee_anim_bp true)
  (bind _assplayer_controller_bp (Utilities|Casting|CastToSPlayerController_bp (Pawn|GetController)))
  (Default|OnDeath _assplayer_controller_bp))

(event EventBeginPlay
  (EventDispatchers|AssignOnDeathRequest (delegate Custom|OnDeathRequest_Event_0))
  (bind _asplayer_controller (Utilities|Casting|CastToPlayerController (Pawn|GetController)))
  (Input|SetInputModeGameOnly _asplayer_controller)
  (Variables|/Script/Engine.PlayerController|SetbShowMouseCursor _asplayer_controller false))

(event EventTick
  (params (DeltaSeconds :type Float%20%28single-precision%29)))

(fn ConstructionScript)