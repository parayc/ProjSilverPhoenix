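; Zip pad actor that pulls a player who enters its sphere toward the pad's static mesh.
; The overlap stores the SPlayer and turns on a flag that makes Tick move them each frame by a lerp from their current location, scaled by delta time and Speed, easing in.
; The live path never clears the flag, prints the position each tick, and leaves its journey fraction unused; an alpha-limited version is disconnected.
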(event OnComponentBeginOverlap(Sphere)
  (params (OverlappedComponent :type Primitive%20Component%20Object%20Reference) (OtherActor :type Actor%20Object%20Reference) (OtherComp :type Primitive%20Component%20Object%20Reference) (OtherBodyIndex :type Integer) (bFromSweep :type Boolean) (SweepResult :type Hit%20Result%20Structure%20%28by%20ref%29))
  (bind _assplayer (Utilities|Casting|CastToSPlayer OtherActor))
  (bind _output_get (Variables|Default|SetOverLapActor _assplayer))
  (Variables|Default|SetStartTime (Utilities|Time|GetTimeSeconds))
  (Variables|Default|SetTotalDistanceTo (Math|Vector|VectorLength (- (Transformation|GetActorLocation _output_get) (Transformation|GetWorldLocation (Variables|Default|GetStaticMesh)))))
  (Variables|Default|SetLerp? true))

(event EventBeginPlay)

(event Collision|EventActorBeginOverlap
  (params (OtherActor :type Actor%20Object%20Reference)))

(event EventTick
  (params (DeltaSeconds :type Float%20%28single-precision%29))
  (Variables|Default|SetTime DeltaSeconds)
  (if (Variables|Default|GetLerp?)
    (Variables|Default|SetCurrentDest (- (Variables|Default|GetStartTime) DeltaSeconds))
    (Variables|Default|SetJourneyFrac (/ (Variables|Default|GetCurrentDest) (Variables|Default|GetTotalDistanceTo)))
    (Development|PrintString (Utilities|String|ToString(Vector) (Math|Vector|Lerp(Vector) (Transformation|GetActorLocation (Variables|Default|GetOverLapActor)) (Transformation|GetWorldLocation (Variables|Default|GetStaticMesh)) (* (Variables|Default|GetTime) (Variables|Default|GetSpeed)))))
    (Transformation|SetActorLocation (Variables|Default|GetOverLapActor) (Math|Vector|Lerp(Vector) (Transformation|GetActorLocation (Variables|Default|GetOverLapActor)) (Transformation|GetWorldLocation (Variables|Default|GetStaticMesh)) (* (Variables|Default|GetTime) (Variables|Default|GetSpeed))) false false)))

(fn ConstructionScript)