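; Bow ranged weapon Blueprint that drives the bow's UI widget as the player draws the bow.
; On BeginPlay it binds to the bow charged and draw end events, which begin and end the widget's UI update respectively.
; The widget reference is lazily fetched from the owning SPlayer's DarkKnightAnim instance and cached for later calls.
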(event Custom|OnDrawBowEnd_Event_0
  (CallFunction|EndBowUIWidget))

(event Custom|OnBowCharged_Event_0
  (CallFunction|PlayBowUIWidget))

(event EventBeginPlay
  (EventDispatchers|AssignOnBowCharged (delegate Custom|OnBowCharged_Event_0))
  (EventDispatchers|AssignOnDrawBowEnd (delegate Custom|OnDrawBowEnd_Event_0)))

(fn ConstructionScript)

(fn PlayBowUIWidget
  (Utilities|IsValid (Variables|UI|GetBowWidgetCrossRef)
    (:Is%20Valid
      (Default|BeginUpdateBowUI (Variables|UI|GetBowWidgetCrossRef)))
    (:Is%20Not%20Valid
      (bind _assplayer (Utilities|Casting|CastToSPlayer (Components|GetOwner)))
      (bind _asdark_knight_anim (Utilities|Casting|CastToDarkKnightAnim (Components|SkeletalMesh|GetAnimInstance (Variables|/Script/Engine.Character|GetMesh _assplayer))))
      (bind _output_get (Variables|UI|SetBowWidgetCrossRef (Variables|/Game/Dynamic/Player/DarkKnightAnimations/DarkKnightAnim.DarkKnightAnim_C|GetBowWidget _asdark_knight_anim)))
      (Default|BeginUpdateBowUI _output_get))))

(fn EndBowUIWidget
  (Utilities|IsValid (Variables|UI|GetBowWidgetCrossRef)
    (:Is%20Valid
      (Default|EndUpdateBowUi (Variables|UI|GetBowWidgetCrossRef)))
    (:Is%20Not%20Valid
      (bind _assplayer (Utilities|Casting|CastToSPlayer (Components|GetOwner)))
      (bind _asdark_knight_anim (Utilities|Casting|CastToDarkKnightAnim (Components|SkeletalMesh|GetAnimInstance (Variables|/Script/Engine.Character|GetMesh _assplayer))))
      (bind _output_get (Variables|UI|SetBowWidgetCrossRef (Variables|/Game/Dynamic/Player/DarkKnightAnimations/DarkKnightAnim.DarkKnightAnim_C|GetBowWidget _asdark_knight_anim)))
      (Default|EndUpdateBowUi _output_get))))