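; Health potion item Blueprint that heals the player's character when it is used from an inventory.
; On BeginPlay it binds a handler to the OnUseItemRequest dispatcher.
; The handler casts the inventory reference's owner to the player controller, gets its controlled pawn as an XBaseCharacter, and adds HealAmount to its current health.
; Tick and the construction script only call the parent, and the overlap event is disabled.
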(event Custom|OnUseItemRequest_Event_0
  (bind _asxbase_character (Utilities|Casting|CastToXBaseCharacter (Pawn|GetControlledPawn (.AsSPlayer%20Controller%20Bp (Utilities|Casting|CastToSPlayerController_bp (Components|GetOwner (Variables|Default|GetInventoryRef)))))))
  (Class|XBaseCharacter|SetAddCurrentHealth _asxbase_character (Variables|Default|GetHeal%20Amount)))

(event EventBeginPlay
  (|CallParentFunction)
  (EventDispatchers|AssignOnUseItemRequest (delegate Custom|OnUseItemRequest_Event_0)))

(event Collision|EventActorBeginOverlap
  (params (OtherActor :type Actor%20Object%20Reference))
  (|CallParentFunction OtherActor))

(event EventTick
  (params (DeltaSeconds :type Float%20%28single-precision%29))
  (|CallParentFunction DeltaSeconds))

(fn ConstructionScript
  (|CallParentFunction))