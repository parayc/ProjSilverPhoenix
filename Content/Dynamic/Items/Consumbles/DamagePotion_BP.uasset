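; Consumable damage potion that temporarily boosts the player's melee damage.
; On activation it shows a sword-power icon in the player UI, caches the current melee weapon's damage modifier and raises it by half.
; On expiry it writes the cached value to whichever melee weapon is then equipped.
; Icon removal and the parent expiry call run only if that weapon check passes.
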(event EventBeginPlay
  (|CallParentFunction))

(event Collision|EventActorBeginOverlap
  (params (OtherActor :type Actor%20Object%20Reference))
  (|CallParentFunction OtherActor))

(event EventTick
  (params (DeltaSeconds :type Float%20%28single-precision%29))
  (|CallParentFunction DeltaSeconds))

(event EventOnActivited
  (params (OwnerController :type Actor%20Object%20Reference) (InventoryRef :type Inventory%20Component%20Object%20Reference))
  (bind _assplayer_controller_bp (Utilities|Casting|CastToSPlayerController_bp OwnerController))
  (bind _assplayer (Utilities|Casting|CastToSPlayer (Pawn|GetControlledPawn _assplayer_controller_bp)))
  (Variables|Default|SetIconRef (Variables|/Game/Dynamic/UI/Player/Player_UI.Player_UI_C|GetIteminUseIcon (Variables|/Game/Dynamic/Player/SPlayerController_bp.SPlayerController_bp_C|GetPlayer_UIWidget _assplayer_controller_bp)))
  (Default|SetIcon (Variables|/Game/Dynamic/UI/Player/Player_UI.Player_UI_C|GetIteminUseIcon (Variables|/Game/Dynamic/Player/SPlayerController_bp.SPlayerController_bp_C|GetPlayer_UIWidget _assplayer_controller_bp)) "/Game/Dynamic/UI/Icons/swords-power.swords-power")
  (bind _output_get (Variables|Default|SetPawnOwner _assplayer))
  (Utilities|IsValid (.currentweapon (Variables|/Script/ProjSilverPhoenix.XBaseCharacter|GetCharacterEquipment _output_get))
    (:Is%20Valid
      (bind _asmelee_weapon (Utilities|Casting|CastToMeleeWeapon (.currentweapon (Variables|/Script/ProjSilverPhoenix.XBaseCharacter|GetCharacterEquipment _output_get))))
      (Variables|Default|SetOriginalDamage (Class|MeleeWeapon|GetDamageModifier _asmelee_weapon))
      (Class|MeleeWeapon|SetDamageModifier _asmelee_weapon (* (Class|MeleeWeapon|GetDamageModifier _asmelee_weapon) 1.5)))))

(event EventOnExpired
  (bind _pawnowner (Variables|Default|GetPawnOwner))
  (bind _characterequipment (Variables|/Script/ProjSilverPhoenix.XBaseCharacter|GetCharacterEquipment _pawnowner))
  (Utilities|IsValid (.currentweapon _characterequipment)
    (:Is%20Valid
      (bind _asmelee_weapon (Utilities|Casting|CastToMeleeWeapon (.currentweapon _characterequipment)))
      (Class|MeleeWeapon|SetDamageModifier _asmelee_weapon (Variables|Default|GetOriginalDamage))
      (Default|RemoveCurrentIcon (Variables|Default|GetIconRef))
      (|CallParentFunction))))

(fn ConstructionScript
  (|CallParentFunction))