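; HealthItem_BP is an item that heals the player who activates it over repeated ticks.
; On activation it casts the owning controller to SPlayerController_bp and stores its controlled SPlayer pawn.
; Each item tick finds that pawn's HealthComponent and, if valid, heals it by a fixed amount.
; Activation and tick also print debug strings, while expiry does nothing.
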(event EventBeginPlay)

(event Collision|EventActorBeginOverlap
  (params (OtherActor :type Actor%20Object%20Reference)))

(event EventTick
  (params (DeltaSeconds :type Float%20%28single-precision%29)))

(event EventOnActivited
  (params (OwnerController :type Actor%20Object%20Reference) (InventoryCompRef :type Inventory%20Component%20Object%20Reference))
  (bind _assplayer_controller_bp (Utilities|Casting|CastToSPlayerController_bp OwnerController))
  (bind _assplayer (Utilities|Casting|CastToSPlayer (Pawn|GetControlledPawn _assplayer_controller_bp)))
  (Variables|Default|SetPawnOwner _assplayer)
  (Development|PrintString "Hello"))

(event EventOnExpired)

(event EventOnItemTick
  (bind _pawnowner (Variables|Default|GetPawnOwner))
  (bind _returnvalue (Actor|GetComponentbyClass _pawnowner "/Script/ProjSilverPhoenix.HealthComponent"))
  (Development|PrintString "tick")
  (Utilities|IsValid _returnvalue
    (:Is%20Valid
      (Class|HealthComponent|Heal _returnvalue 5.0))))

(fn ConstructionScript)